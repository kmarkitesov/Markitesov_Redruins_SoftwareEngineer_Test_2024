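; Character that rides along a BP_Trajectory spline and launches physics balls along a predicted ballistic arc.
; A timeline, re-triggered on finish, sets location and tangent-based rotation, with its play rate driven by an adjustable MovementSpeed.
; While aiming, Tick steps the projectile equation from view-direction velocity until below Z=0, drawing debug spheres and moving a hit marker.
; ReleaseProjectile hides the preview and spawns BP_PhysicBall at the first path point with that velocity.
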(event `self.ReceiveBeginPlay`
  (bind _returnvalue (`GameplayStatics.GetActorOfClass` "/Game/Task_05/BP_Trajectory.BP_Trajectory_C"))
  (set `self.MovementTrajectory` _returnvalue)
  (`self.PlayTimeline`)
  (bind _returnvalue_2 (`|SpawnActorFromClass` "/Game/Task_05/BP_HitPlace.BP_HitPlace_C" (`self.HitPlaceTransform`) "Undefined" "MultiplyWithRoot" null null))
  (set `self.HitPlace` _returnvalue_2))

(event `self.ReceiveTick`
  (params (DeltaSeconds :type "Float (single-precision)"))
  (`TimelineComponent.SetPlayRate` (`self.Timeline`) (`self.MovementSpeed`))
  (set `self.LaunchVelocity` (* (`.Rotation` (`Controller.GetPlayerViewPoint` (`GameplayStatics.GetPlayerController` 0))) (`self.LaunchSpeed`)))
  (if (`self.IsTrajectoryShowing`)
    (`self.PredictTrajectory` DeltaSeconds)))

(event `PlayTimeline`
  (bind _spline (`/Game/Task_05/BP_Trajectory.Spline` (`self.MovementTrajectory`)))
  (bind (_direction _progress) (`Timeline|Timeline`)
    (:`Update`
      (bind _returnvalue (* _progress (`SplineComponent.GetSplineLength` (`/Game/Task_05/BP_Trajectory.Spline` (`self.MovementTrajectory`)))))
      (`self.K2_SetActorLocationAndRotation` (`SplineComponent.GetLocationAtDistanceAlongSpline` _spline _returnvalue "World") (`KismetMathLibrary.Conv_VectorToRotator` (`SplineComponent.GetTangentAtDistanceAlongSpline` _spline _returnvalue "World"))))
    (:`Finished`
      (`self.PlayTimeline`))))

(fn `CalculateTrajectoryPoint`
  (params (StartLocation :type "Vector Structure") (LaunchVelocity :type "Vector Structure") (Gravity :type "Float (double-precision)") (Time :type "Float (double-precision)"))
  (returns (Position :type "Vector Structure"))
  (locals (TrajectoryPointPosition :type "Vector Structure" :default (0.0 0.0 0.0)))
  (bind (_launchvelocity_x _launchvelocity_y) (`KismetMathLibrary.BreakVector` (`local.LaunchVelocity`)))
  (bind (_startlocation_x _startlocation_y _startlocation_z) (`KismetMathLibrary.BreakVector` (`local.StartLocation`)))
  (bind (_launchvelocity_x_2 _launchvelocity_y_2 _launchvelocity_z) (`KismetMathLibrary.BreakVector` (`local.LaunchVelocity`)))
  (bind _startlocation_x_2 (`KismetMathLibrary.BreakVector` (`local.StartLocation`)))
  (bind _launchvelocity_x_3 (`KismetMathLibrary.BreakVector` (`local.LaunchVelocity`)))
  (bind (_startlocation_x_3 _startlocation_y_2) (`KismetMathLibrary.BreakVector` (`local.StartLocation`)))
  (bind _output_get (set `local.TrajectoryPointPosition` (`KismetMathLibrary.MakeVector` (+ _startlocation_x_2 (* _launchvelocity_x_3 (`local.Time`))) (+ _startlocation_y_2 (* _launchvelocity_y (`local.Time`))) (+ _startlocation_z (* _launchvelocity_z (`local.Time`)) (* 0.5 (`local.Gravity`) (`KismetMathLibrary.Square` (`local.Time`)))))))
  (return _output_get))

(fn `ChangeCurrentSpeed`
  (params (NewSpeed :type "Float (double-precision)"))
  (set `self.MovementSpeed` (+ NewSpeed (`self.MovementSpeed`))))

(fn `PredictTrajectory`
  (params (DeltaSeconds :type "Float (double-precision)"))
  (locals (StartLocation :type "Vector Structure") (CurrentVelocity :type "Vector Structure") (PathPoints :type "Array of Vector Structure") (TimeStep :type "Float (double-precision)" :default 0.08) (CurrentTime :type "Float (double-precision)") (TrajectoryPointLocation :type "Vector Structure"))
  (bind _pathpoints (`local.PathPoints`))
  (bind (_trajectorypointlocation_x _trajectorypointlocation_y _trajectorypointlocation_z) (`KismetMathLibrary.BreakVector` (`local.TrajectoryPointLocation`)))
  (set `local.StartLocation` (`self.K2_GetActorLocation`))
  (set `local.CurrentVelocity` (`self.LaunchVelocity`))
  (while (>= _trajectorypointlocation_z 0.0)
    (set `local.CurrentTime` (+ (`local.CurrentTime`) (`local.TimeStep`)))
    (bind _position (`self.CalculateTrajectoryPoint` (`local.StartLocation`) (`local.CurrentVelocity`) (`MovementComponent.GetGravityZ` (`self.CharacterMovement`)) (`local.CurrentTime`)))
    (bind _output_get (set `local.TrajectoryPointLocation` _position))
    (`KismetArrayLibrary.Array_Add` (`local.PathPoints`) _output_get)
    (`KismetSystemLibrary.DrawDebugSphere` (`local.TrajectoryPointLocation`) 10.0 12 (struct :`R` 1.0 :`B` 0.075037 :`A` 1.0)))
  (set `self.LaunchPosition` (`|GetArrayItem` (`local.PathPoints`)))
  (`self.K2_SetActorLocation` (`self.HitPlace`) (`KismetMathLibrary.MakeVector` (.x (`|GetArrayItem` _pathpoints (`KismetArrayLibrary.Array_LastIndex` _pathpoints))) (.y (`|GetArrayItem` _pathpoints (`KismetArrayLibrary.Array_LastIndex` _pathpoints)))) false false))

(fn `ReleaseProjectile`
  (if (`self.IsTrajectoryShowing`)
    (set `self.IsTrajectoryShowing` false)
    (bind _returnvalue (`|SpawnActorFromClass` "/Game/Task_05/BP_PhysicBall.BP_PhysicBall_C" (`KismetMathLibrary.MakeTransform` (`self.LaunchPosition`) (struct) (0.3 0.3 0.3)) "Undefined" "MultiplyWithRoot" null null))
    (`PrimitiveComponent.AddImpulse` (`/Game/Task_05/BP_PhysicBall.Sphere` _returnvalue) (`self.LaunchVelocity`) "None" true)))

(fn `UserConstructionScript`)