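; Character that detects interactable actors in its line of sight, shows their interact label and sends them interact messages.
; Two Visibility traces, from the camera view point and the top of the capsule, must hit the same actor.
; Tick toggles the widget on BP_Task_01_Actor instances cached at BeginPlay.
; CheckForInteractable fires OnInteract for BPI_Interact targets, and its bound handler calls InteractMessage on them.
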(event `HandleInteract_Event` :!signature `self.OnInteract`
  (params (InteractedActor :type "Actor Object Reference"))
  (`self.HandleInteract` InteractedActor))

(event `self.ReceiveBeginPlay`
  (add `self.OnInteract` (delegate `HandleInteract_Event`))
  (bind _outactors (`GameplayStatics.GetAllActorsOfClass` "/Game/Task_01/Blueprints/BP_Task_01_Actor.BP_Task_01_Actor_C"))
  (set `self.Interactables` _outactors))

(event `self.ReceiveTick`
  (params (DeltaSeconds :type "Float (single-precision)"))
  (bind _hitactor (`self.TraceLineOfSight`))
  (`/Engine/EditorBlueprintResources/StandardMacros.IsValid` _hitactor
    (:`Is Valid`
      (bind _asbp_task_01_actor (cast `/Game/Task_01/Blueprints/BP_Task_01_Actor` _hitactor)
        (:`then`
          (if (`KismetArrayLibrary.Array_Contains` (`self.Interactables`) _asbp_task_01_actor)
            (`Widget.SetVisibility` (`WidgetComponent.GetWidget` (`/Game/Task_01/Blueprints/BP_Task_01_Actor.InteractWidget` _asbp_task_01_actor)) "HitTestInvisible")
            (set `self.CurrentInteractable` _asbp_task_01_actor)
            (else
              (`self.SetHiddenInteractLabel`))))
        (:`CastFailed`
          (`self.SetHiddenInteractLabel`))))
    (:`Is Not Valid`
      (`self.SetHiddenInteractLabel`))))

(fn `CheckForInteractable`
  (locals (HitActor :type "Actor Object Reference"))
  (bind _hitactor (`self.TraceLineOfSight`))
  (set `local.HitActor` _hitactor)
  (bind _hitactor_2 (`local.HitActor`)
    (:`then`
      (if true
        (if (`KismetSystemLibrary.DoesImplementInterface` _hitactor_2 "/Game/Task_01/Blueprints/BPI_Interact.BPI_Interact_C")
          (`self.OnInteract` (`local.HitActor`)))))
    (:`else`)))

(fn `HandleInteract`
  (params (InteractedActor :type "Actor Object Reference"))
  (if (`KismetSystemLibrary.DoesImplementInterface` InteractedActor "/Game/Task_01/Blueprints/BPI_Interact.BPI_Interact_C")
    (message `/Game/Task_01/Blueprints/BPI_Interact.Interact` InteractedActor)))

(fn `SetHiddenInteractLabel`
  (`/Engine/EditorBlueprintResources/StandardMacros.IsValid` (`self.CurrentInteractable`)
    (:`Is Valid`
      (`Widget.SetVisibility` (`WidgetComponent.GetWidget` (`/Game/Task_01/Blueprints/BP_Task_01_Actor.InteractWidget` (`self.CurrentInteractable`))) "Hidden")
      (set `self.CurrentInteractable` null))))

(fn `TraceLineOfSight`
  (returns (HitActor :type "Actor Object Reference"))
  (bind (_location _rotation) (`Controller.GetPlayerViewPoint` (`self.GetController`)))
  (bind (_location_2 _rotation_2) (`Controller.GetPlayerViewPoint` (`self.GetController`)))
  (bind (_location_3 _rotation_3) (`Controller.GetPlayerViewPoint` (`self.GetController`)))
  (bind _outhit (`KismetSystemLibrary.LineTraceSingle` :`Start` (+ (+ (`self.K2_GetActorLocation`) (`KismetMathLibrary.MakeVector` 0.0 0.0 (`CapsuleComponent.GetScaledCapsuleHalfHeight` (`self.CapsuleComponent`)))) (`self.GetActorForwardVector`)) :`End` (+ _location_3 (* (`KismetMathLibrary.Conv_RotatorToVector` _rotation_3) (`self.LineOfSightDistance`))) :`TraceChannel` "TraceTypeQuery1" :`DrawTime` 2.0))
  (bind _outhit_2 (`KismetSystemLibrary.LineTraceSingle` :`Start` (+ _location (`KismetMathLibrary.Conv_RotatorToVector` _rotation)) :`End` (+ _location_2 (* (`KismetMathLibrary.Conv_RotatorToVector` _rotation_2) (`self.LineOfSightDistance`))) :`TraceChannel` "TraceTypeQuery1" :`TraceColor` (struct :`R` 0.345032 :`G` 0.262768 :`B` 1.0 :`A` 1.0) :`TraceHitColor` (struct :`G` 0.217532 :`B` 1.0 :`A` 1.0)))
  (bind (_bblockinghit _binitialoverlap _time _distance _location_4 _impactpoint _normal _impactnormal _physmat _hitactor) (`GameplayStatics.BreakHitResult` _outhit_2))
  (if (== _hitactor (`.HitActor` (`GameplayStatics.BreakHitResult` _outhit)))
    (return _hitactor)))

(fn `UserConstructionScript`)