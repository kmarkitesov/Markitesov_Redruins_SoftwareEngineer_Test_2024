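; BP_Task_01_Actor is an interactable world actor with a distance marker widget and a sphere mesh.
; On BeginPlay it caches the player character and the W_Marker instance from its widget component.
; Every Tick it measures distance to the player, hiding the marker inside a minimum range and otherwise showing it with the updated distance.
; Its Interact event swaps the sphere's material.
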(event `self.ReceiveBeginPlay`
  (bind _returnvalue (`GameplayStatics.GetPlayerCharacter` 0))
  (`/Engine/EditorBlueprintResources/StandardMacros.IsValid` _returnvalue
    (:`Is Valid`
      (bind _asbp_task_01_character (cast `/Game/Task_01/Blueprints/BP_Task_01_Character` _returnvalue))
      (set `self.PlayerCharacter` _asbp_task_01_character)
      (bind _asw_marker (cast `/Game/Task_01/Widgets/W_Marker` (`WidgetComponent.GetUserWidgetObject` (`self.MarkerWidget`))))
      (set `self.MarkerWidgetReference` _asw_marker))))

(event `self.ReceiveTick`
  (params (DeltaSeconds :type "Float (single-precision)"))
  (bind _output_get (set `self.ObjectToCharacterDistance` (`self.GetDistanceTo` (`self.PlayerCharacter`))))
  (if (< _output_get (`self.MinDistanceForMarkerVisibility`))
    (`Widget.SetVisibility` (`self.MarkerWidgetReference`) "Hidden")
    (else
      (`Widget.SetVisibility` (`self.MarkerWidgetReference`) "Visible")
      (`/Game/Task_01/Widgets/W_Marker.Update Distance` (`self.MarkerWidgetReference`) (`self.ObjectToCharacterDistance`)))))

(event `/Game/Task_01/Blueprints/BPI_Interact.Interact`
  (`PrimitiveComponent.SetMaterial` (`self.Sphere`) 0 (`self.Material`)))

(fn `UserConstructionScript`)